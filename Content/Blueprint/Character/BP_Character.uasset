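; BP_Character is a character Blueprint that sets up on-screen UI and keeps its health display current.
; On BeginPlay it adds crosshair and HUD widgets to the viewport, stores the HUD reference and seeds it with current and default health from its Health component.
; AnyDamage only refreshes the HUD from that component; this graph does not change health itself.
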(event EventBeginPlay
  (bind _health (Variables|Default|GetHealth))
  (bind _returnvalue (UserInterface|CreateWidget "/Game/WBP/WBP_Crosshair.WBP_Crosshair_C"))
  (UserInterface|Viewport|AddtoViewport _returnvalue 0)
  (bind _returnvalue_2 (UserInterface|CreateWidget "/Game/WBP/WBP_HUD.WBP_HUD_C"))
  (bind _output_get (Variables|Default|SetHUD_Ref _returnvalue_2))
  (UserInterface|Viewport|AddtoViewport _output_get 0)
  (Default|UpdateHealth (Variables|Default|GetHUD_Ref) (Variables|/Script/Test.HealthComponent|GetHealth _health) (Variables|/Script/Test.HealthComponent|GetDefaultHealth _health)))

(event Game|Damage|EventAnyDamage
  (params (Damage :type Float%20%28single-precision%29) (DamageType :type Damage%20Type%20Object%20Reference) (InstigatedBy :type Controller%20Object%20Reference) (DamageCauser :type Actor%20Object%20Reference))
  (bind _health (Variables|Default|GetHealth))
  (Default|UpdateHealth (Variables|Default|GetHUD_Ref) (Variables|/Script/Test.HealthComponent|GetHealth _health) (Variables|/Script/Test.HealthComponent|GetDefaultHealth _health)))

(fn ConstructionScript)